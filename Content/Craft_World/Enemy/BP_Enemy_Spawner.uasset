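; BP_Enemy_Spawner is an actor that repeatedly spawns waves of enemies at its own location.
; BeginPlay calls the spawn event with the Enemy class, the actor's transform and the NumberOfEnemy count.
; The event spawns that many actors at the same transform, waits for the SpawnDealy delay, then calls itself again, with no stop condition.
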(event `self.ReceiveBeginPlay`
  ;[1 1 1] Enemy Spawner
  (`self.Spawn_Enemy` (`self.Enemy`) (`self.GetTransform`) (`self.Number Of Enemy`)))

(event `Spawn_Enemy`
  (params (Enemy :type "Actor Class Reference") (SpawnTransform :type "Transform Structure") (`Number of Enemy` :type Integer))
  ;[1 1 1] Enemy Spawner
  (for _ (range `Number of Enemy`)
    (`|SpawnActorFromClass` Enemy SpawnTransform "Undefined" "MultiplyWithRoot" null null))
  (`KismetSystemLibrary.Delay` (`self.Spawn Dealy`))
  (`self.Spawn_Enemy` (`self.Enemy`) (`self.GetTransform`) (`self.Number Of Enemy`)))

(fn `UserConstructionScript`)