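; BP_Rock is a rock actor that acts as either a pickup or a hidden spot that reveals a rock, chosen by RockCollectable.
; Mode 0 hides the mesh on BeginPlay, then shows it with a drop sound on box overlap, leaving HasRock false so it can repeat.
; Mode 1 hides the mesh on overlap with the same sound and sets HasRock, blocking repeats.
; Overlaps are not filtered by actor.
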(event `self.Box.OnComponentBeginOverlap`
  (params (OverlappedComponent :type "PrimitiveComponent Object Reference") (OtherActor :type "Actor Object Reference") (OtherComp :type "PrimitiveComponent Object Reference") (OtherBodyIndex :type Integer) (bFromSweep :type Boolean) (SweepResult :type "HitResult Structure (by ref)"))
  (`|ExecutionSequence`
    (:`then_0`
      (if (== (`self.Rock_Collectable?`) 0)
        (if (not (`self.Has_Rock?`))
          (`SceneComponent.SetVisibility` (`self.SM_Rock_Collectable`) true false)
          (`GameplayStatics.PlaySound2D` "/Game/Craft_World/Sound/Rock_Drop_1.Rock_Drop_1" 1.0 1.0 0.0 null null)
          (set `self.Has_Rock?` false))))
    (:`then_1`
      (if (== (`self.Rock_Collectable?`) 1)
        (if (not (`self.Has_Rock?`))
          (`SceneComponent.SetVisibility` (`self.SM_Rock_Collectable`) false false)
          (`GameplayStatics.PlaySound2D` "/Game/Craft_World/Sound/Rock_Drop_1.Rock_Drop_1" 1.0 1.0 0.0 null null)
          (set `self.Has_Rock?` true))))))

(event `self.ReceiveBeginPlay`
  (`/Engine/EditorBlueprintResources/StandardMacros.DoOnce` false
    (:`Completed`
      (if (== (`self.Rock_Collectable?`) 0)
        (`SceneComponent.SetVisibility` (`self.SM_Rock_Collectable`) false false)))))

(fn `UserConstructionScript`)