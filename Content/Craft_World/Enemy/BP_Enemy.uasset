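; BP_Enemy is an enemy character that endlessly chases the player with AIMoveTo, restarting on success or failure.
; Capsule overlaps apply contact damage, and a ChangeSpeed event raises walk speed within a clamped range.
; Taking damage briefly halts movement for a hit montage.
; Death disables movement and collision, increments the player's kill count, randomly drops an ammo crate and destroys the actor after a delay.
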(event `self.ReceiveBeginPlay`
  ;[1 1 1] Chase_Player
  (bind _asue_4asp_character (cast `/Game/Craft_World/Charater/Ue4ASP_Character` (`GameplayStatics.GetPlayerCharacter` 0)))
  (bind _output_get (set `self.Char_REF` _asue_4asp_character))
  (`self.Chase_Player` _output_get))

(event `Chase_Player`
  (params (`Player to chase` :type "/Game/Craft_World/Charater/Ue4ASP_Character Object Reference"))
  ;[1 1 1] Chase_Player
  (`|AIMoveTo` self (0.0 0.0 0.0) `Player to chase`
    (:`OnSuccess`
      _)
    (:`OnFail`
      _))
  (`self.Chase_Player` (`self.Char_REF`)))

(event `/Game/Craft_World/Speed_Interface.Change Speed`
  (bind _charactermovement (`self.CharacterMovement`))
  ;[1 1 1] AI_Speed_System
  (set `CharacterMovementComponent.MaxWalkSpeed` (`KismetMathLibrary.FClamp` (+ (`CharacterMovementComponent.MaxWalkSpeed` _charactermovement) 100.0) 400.0 1000.0) _charactermovement))

(event `self.ReceiveAnyDamage`
  (params (Damage :type "Float (single-precision)") (DamageType :type "DamageType Object Reference") (InstigatedBy :type "Controller Object Reference") (DamageCauser :type "Actor Object Reference"))
  (bind _returnvalue (`self.K2_GetActorLocation`))
  ;[1 1 1] AI_Danage & Dead_System
  (if (not (`self.Is Dead?`))
    (bind _output_get (set `self.Health` (`KismetMathLibrary.FClamp` (- (`self.Health`) Damage) 0.0 100.0)))
    (if (== _output_get 0.0)
      (`GameplayStatics.PlaySoundAtLocation` "/Game/Craft_World/Sound/DeathScream_1.DeathScream_1" _returnvalue (struct) 1.0 1.0 0.0 null null null null)
      (`CharacterMovementComponent.DisableMovement` (`self.CharacterMovement`))
      (set `self.Is Dead?` true)
      (`self.PlayAnimMontage` "/Game/Craft_World/Charater/Animations/Death_2_Montage.Death_2_Montage")
      (`PrimitiveComponent.SetCollisionEnabled` (`self.CapsuleComponent`) "NoCollision")
      (`|ExecutionSequence`
        (:`then_0`
          (bind _asue_4asp_character (cast `/Game/Craft_World/Charater/Ue4ASP_Character` (`GameplayStatics.GetPlayerCharacter` 0)))
          (`/Engine/EditorBlueprintResources/StandardMacros.IncrementInt` (`/Game/Craft_World/Charater/Ue4ASP_Character.Kills_Count` _asue_4asp_character)
            (:`  `
              (if (`KismetMathLibrary.RandomBoolWithWeight` 0.5)
                (`|SpawnActorFromClass` "/Game/Craft_World/Guns/BP_Ammo_Create.BP_Ammo_Create_C" (`KismetMathLibrary.MakeTransform` (- (`self.K2_GetActorLocation`) (0.0 0.0 85.0))) "Undefined" "MultiplyWithRoot" null null)))))
        (:`then_1`
          (`KismetSystemLibrary.Delay` 10.0)
          (`self.K2_DestroyActor`)))
      (else
        (`GameplayStatics.PlaySoundAtLocation` "/Game/Craft_World/Sound/DamageCUE.DamageCUE" _returnvalue (struct) 1.0 1.0 0.0 null null null null)
        (`CharacterMovementComponent.DisableMovement` (`self.CharacterMovement`))
        (set `self.Is Dead?` false)
        (bind _returnvalue_2 (`self.PlayAnimMontage` "/Game/Craft_World/Charater/Animations/Hit_1_Montage.Hit_1_Montage"))
        (`KismetSystemLibrary.Delay` _returnvalue_2)
        (if (not (`self.Is Dead?`))
          (`CharacterMovementComponent.SetMovementMode` (`self.CharacterMovement`) "MOVE_Walking" 0))))))

(event `self.Capsule.OnComponentBeginOverlap`
  (params (OverlappedComponent :type "PrimitiveComponent Object Reference") (OtherActor :type "Actor Object Reference") (OtherComp :type "PrimitiveComponent Object Reference") (OtherBodyIndex :type Integer) (bFromSweep :type Boolean) (SweepResult :type "HitResult Structure (by ref)"))
  ;[1 1 1] AI_Damage_System
  (`GameplayStatics.ApplyDamage` OtherActor 1.0 null self)
  (`GameplayStatics.PlaySound2D` "/Game/Craft_World/Sound/DamageCUE.DamageCUE" 1.0 1.0 0.0 null null))

(fn `UserConstructionScript`)