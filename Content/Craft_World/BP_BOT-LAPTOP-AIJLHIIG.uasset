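; An AI bot that patrols a level, chases pawns it sees and damages the player.
; BeginPlay starts an endless four-corner AI MoveTo loop with hard-coded points; PawnSensing triggers a chase, then restarts patrol after a retriggerable delay.
; Any capsule overlap damages player 0 and plays a sound, without checking the overlapping actor.
; ChangeSpeed raises walk speed up to a cap; a self-repeating random patrol exists but is not started here.
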(event `self.ReceiveBeginPlay`
  ;[1 1 1] Event Being Play
  (`|ExecutionSequence`
    (:`then_0`
      (`self.AI_Patrol`))))

(event `AI_Random_Patrol`
  ;[1 1 1] AI_Random_Patrol
  (`|AIMoveTo` self (`NavigationSystemV1.K2_GetRandomReachablePointInRadius` (`self.K2_GetActorLocation`) 1500.0 null null) null
    (:`OnSuccess`
      (`self.AI_Random_Patrol`))))

(event `AI_Patrol`
  ;[1 1 1] AI_Patrol System
  (`|AIMoveTo` self (200.0 3300.0 10.0) null :!label _label
    (:`OnSuccess`
      (`|AIMoveTo` self (2800.0 3300.0 10.0) null
        (:`OnSuccess`
          (`|AIMoveTo` self (2800.0 200.0 10.0) null
            (:`OnSuccess`
              (`|AIMoveTo` self (200.0 200.0 10.0) null
                (:`OnSuccess`
                  (goto _label))))))))))

(event `self.PawnSensing.OnSeePawn`
  (params (Pawn :type "Pawn Object Reference"))
  ;[1 1 1] AI_Chase_System
  (`|ExecutionSequence`
    (:`then_0`
      (`|AIMoveTo` self (0.0 0.0 0.0) Pawn))
    (:`then_1`
      (`KismetSystemLibrary.RetriggerableDelay` 2.0)
      (`self.AI_Patrol`))))

(event `self.Capsule.OnComponentBeginOverlap`
  (params (OverlappedComponent :type "PrimitiveComponent Object Reference") (OtherActor :type "Actor Object Reference") (OtherComp :type "PrimitiveComponent Object Reference") (OtherBodyIndex :type Integer) (bFromSweep :type Boolean) (SweepResult :type "HitResult Structure (by ref)"))
  ;[1 1 1] AI_Damage_System
  (`GameplayStatics.ApplyDamage` (`GameplayStatics.GetPlayerCharacter` 0) 10.0 null self)
  (`GameplayStatics.SpawnSound2D` "/Game/Craft_World/Sound/DamageCUE.DamageCUE" 1.0 1.0 0.0 null))

(event `/Game/Craft_World/Speed_Interface.Change Speed`
  (bind _charactermovement (`self.CharacterMovement`))
  ;[1 1 1] AI_Speed_System
  (set `CharacterMovementComponent.MaxWalkSpeed` (`KismetMathLibrary.FClamp` (+ (`CharacterMovementComponent.MaxWalkSpeed` _charactermovement) 100.0) 0.0 1000.0) _charactermovement))

(fn `UserConstructionScript`)